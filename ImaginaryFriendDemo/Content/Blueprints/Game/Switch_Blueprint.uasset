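; A switch Blueprint that opens a door when the player presses Use inside its trigger box.
; Overlap enables input and shows a prompt based on whether the door is open; leaving disables input and hides it.
; Pressing Use rescales an actor, moves it to a hardcoded location, swaps the prompt and plays a timeline.
; The timeline rotates ChestDoor by adding its track to a cached forward vector and converting that to a rotation.
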(event `self.ReceiveBeginPlay`)

(event `self.ReceiveTick`
  (params (DeltaSeconds :type "Float (single-precision)")))

(event `ReceiveBeginPlay_Copy`
  ;[1 1 1] Sets the rotation for the exit door
  (set `self.Door Rotation` (`KismetMathLibrary.Conv_RotatorToVector` (`self.K2_GetActorRotation`))))

(event `self.Trigger Box.OnComponentBeginOverlap`
  (params (OtherActor :type "Actor Object Reference") (OtherComp :type "PrimitiveComponent Object Reference") (OtherBodyIndex :type Integer) (bFromSweep :type Boolean) (SweepResult :type "EngineTypes.HitResult Structure (by ref)"))
  ;[1 1 1] When Player Overlaps with Trigger Box, this determines what text is displayed
  (set `self.Overlap` true)
  (`self.EnableInput` (`GameplayStatics.GetPlayerController` 0))
  (if (`self.Open Door`)
    (`SceneComponent.SetVisibility` true)
    (else
      (`SceneComponent.SetVisibility` true))))

(event `self.Trigger Box.OnComponentEndOverlap`
  (params (OtherActor :type "Actor Object Reference") (OtherComp :type "PrimitiveComponent Object Reference") (OtherBodyIndex :type Integer))
  ;[1 1 1] When Player Overlaps with Trigger Box, this determines what text is displayed
  (set `self.Overlap` false)
  (`self.DisableInput` (`GameplayStatics.GetPlayerController` 0))
  (`SceneComponent.SetVisibility` false)
  (`SceneComponent.SetVisibility` false))

(event `InputAction|ActionUse`
  ;[1 1 1] Opens Door if Box if Overlapped and Player Presses E
  (:`Pressed`
    (bind _output_get (set `self.E Pressed` true))
    (if (and _output_get (`self.Overlap`))
      (`self.SetActorScale3D` (0.15 0.15 0.15))
      (`self.K2_SetActorLocation` (-1936.0 341.0 778.5))
      (set `self.E Pressed` false)
      (`SceneComponent.SetVisibility` false)
      (set `self.Open Door` true)
      (`SceneComponent.SetVisibility` true)
      (bind (_direction _newtrack_1) (`Timeline|Timeline_0`)
        (:`Update`
          (`self.SetActorRotation` (`self.Chest Door`) (`KismetMathLibrary.Conv_VectorToRotator` (+ _newtrack_1 (`self.Door Rotation`)))))))))

(fn `UserConstructionScript`)